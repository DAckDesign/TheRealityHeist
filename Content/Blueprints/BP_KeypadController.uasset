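; BP_KeypadController is a keypad controller that builds an entered code and checks it against a stored code.
; AddNumber appends each received key to CurrentCode and shows it on a TextRender, routing "Clr" and "Ent" keys to Clear and Enter.
; Clear empties the code and hides the SpotLight, while Enter shows it green for a match or red for a mismatch.
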(event Custom|AddNumber
  (params (ReceivedNumber :type Text))
  (bind _returnvalue (Utilities|String|ToString(Text) ReceivedNumber))
  (switch string _returnvalue
    (:Default
      (bind _output_get (Variables|Default|SetCurrentCode (Utilities|Text|ToText(String) (Utilities|String|Append (Utilities|String|ToString(Text) (Variables|Default|GetCurrentCode)) _returnvalue))))
      (Rendering|Components|TextRender|SetText (Variables|Default|GetTextRender) _output_get))
    (:Clr
      (CallFunction|Clear))
    (:Ent
      (CallFunction|Enter))))

(event Custom|Clear
  (Variables|Default|SetCurrentCode "")
  (Rendering|SetVisibility (Variables|Default|GetSpotLight) false false)
  (Rendering|Components|TextRender|SetText (Variables|Default|GetTextRender) (stale Custom|AddNumber _output_get)))

(event Custom|Enter
  (bind _spotlight (Variables|Default|GetSpotLight))
  (if (Utilities|Enum|Equal(Enum) (Variables|Default|GetCurrentCode) (Variables|Default|GetCode))
    (Rendering|Components|Light|SetLightColor _spotlight "(R=0.000000,G=1.000000,B=0.000000,A=1.000000)" true)
    (else
      (Rendering|Components|Light|SetLightColor (Variables|Default|GetSpotLight) "(R=1.000000,G=0.000000,B=0.000000,A=1.000000)" true)))
  (Rendering|SetVisibility _spotlight true false))

(event EventBeginPlay)

(event Collision|EventActorBeginOverlap
  (params (OtherActor :type Actor%20Object%20Reference)))

(event EventTick
  (params (DeltaSeconds :type Float%20%28single-precision%29)))

(fn ConstructionScript)
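; BP_Safe_Lock is a rotatable safe lock that the player turns with a hand.
; Press stores the acting hand's mesh and its starting world roll, and Unpress stops the rotation.
; While held, Tick sums the hand's current and initial roll and applies it as the actor's relative pitch, with roll and yaw zeroed.
; It contains no combination or unlock logic.
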(event EventBeginPlay)

(event Collision|EventActorBeginOverlap
  (params (OtherActor :type Actor%20Object%20Reference)))

(event EventTick
  (params (DeltaSeconds :type Float%20%28single-precision%29))
  (if (Variables|Default|GetIsRotating)
    (bind _output_get (Variables|Default|SetCurrentHandRotation (+ (.roll (Transformation|GetWorldRotation (Variables|Default|GetPickingHand))) (Variables|Default|GetInitialHandRotation))))
    (Transformation|SetActorRelativeRotation (Math|Rotator|MakeRotator 0.0 _output_get 0.0))))

(event EventPress
  (params (ActingHand :type BP%20Motion%20Controller%20Object%20Reference))
  (bind _output_get (Variables|Default|SetPickingHand (Variables|/Game/VirtualRealityBP/Blueprints/BP_MotionController.BP_MotionController_C|GetHandMesh ActingHand)))
  (Variables|Default|SetInitialHandRotation (.roll (Transformation|GetWorldRotation _output_get)))
  (Variables|Default|SetIsRotating true))

(event EventUnpress
  (Variables|Default|SetIsRotating false))

(fn ConstructionScript)
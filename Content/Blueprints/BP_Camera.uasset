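; BP_Camera is a swinging security camera that flags a Wheel and a Lock as observed and can sound an alarm.
; A timeline started on BeginPlay sweeps the camera's yaw around a fixed offset.
; Capsule overlaps set and clear each target's IsObserved flag.
; Tick plays the alarm once when Gotcha is true, while a separate ActivateSound event plays the camera sound.
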(event OnComponentBeginOverlap(Capsule)
  (params (OverlappedComponent :type Primitive%20Component%20Object%20Reference) (OtherActor :type Actor%20Object%20Reference) (OtherComp :type Primitive%20Component%20Object%20Reference) (OtherBodyIndex :type Integer) (bFromSweep :type Boolean) (SweepResult :type Hit%20Result%20Structure%20%28by%20ref%29))
  (bind _wheel (Variables|Default|GetWheel))
  (bind _lock (Variables|Default|GetLock))
  (if (== OtherActor _wheel)
    (Variables|/Game/BP_safe_wheel.BP_safe_wheel_C|SetIsObserved _wheel true)
    (elif (== OtherActor _lock)
      (Variables|/Game/Blueprints/BP_Safe_Lock.BP_Safe_Lock_C|SetIsObserved _lock true))))

(event OnComponentEndOverlap(Capsule)
  (params (OverlappedComponent :type Primitive%20Component%20Object%20Reference) (OtherActor :type Actor%20Object%20Reference) (OtherComp :type Primitive%20Component%20Object%20Reference) (OtherBodyIndex :type Integer))
  (bind _wheel (Variables|Default|GetWheel))
  (bind _lock (Variables|Default|GetLock))
  (if (== OtherActor _wheel)
    (Variables|/Game/BP_safe_wheel.BP_safe_wheel_C|SetIsObserved _wheel false)
    (elif (== OtherActor _lock)
      (Variables|/Game/Blueprints/BP_Safe_Lock.BP_Safe_Lock_C|SetIsObserved _lock false))))

(event Custom|ActivateSound
  (Audio|Components|Audio|Play (Variables|Default|GetCameraSound) 0.0))

(event EventBeginPlay
  (bind _rollingamount (Timeline|CameraSwinging PlayFromStart)
    (:Update
      (Transformation|SetRelativeRotation (Variables|Default|GetCamera) (Math|Rotator|MakeRotator 2e+01 0.0 (+ _rollingamount 4e+01)) false false))))

(event Collision|EventActorBeginOverlap
  (params (OtherActor :type Actor%20Object%20Reference)))

(event EventTick
  (params (DeltaSeconds :type Float%20%28single-precision%29))
  (if (Variables|Default|GetGotcha!)
    (Utilities|FlowControl|DoOnce false
      (:Completed
        (Audio|Components|Audio|Play (Variables|Default|GetAlarm) 0.0)))))

(fn ConstructionScript)
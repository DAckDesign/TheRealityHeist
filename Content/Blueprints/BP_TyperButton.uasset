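; BP_TyperButton is a configurable keypad button that sends its number to a controller when pressed.
; The construction script sets its label, mesh and tone sound from variables.
; Press plays a timeline that moves the mesh along relative Y, calls AddNumber on the Controller, and plays a typewriter click with the tone.
; IsUsed swaps the mesh to a clicked material; the point light toggle is unconnected.
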(event Custom|IsUsed
  (Rendering|Material|SetMaterial (Variables|Components|GetMesh) 0 "/Game/Meshes/Materials/Mat_Keypad/Mat_Keypad_Pivot_Clicked.Mat_Keypad_Pivot_Clicked"))

(event EventBeginPlay)

(event Collision|EventActorBeginOverlap
  (params (OtherActor :type Actor%20Object%20Reference)))

(event EventPress
  (params (ActingHand :type BP%20Motion%20Controller%20Object%20Reference))
  (Utilities|FlowControl|Sequence
    (:then_0
      (bind _buttonposition (Timeline|ButtonPressingAnim PlayFromStart)
        (:Update
          (Transformation|SetRelativeTransform (Variables|Components|GetMesh) (Math|Transform|MakeTransform (Math|Vector|MakeVector 0.0 _buttonposition 0.0) "0, 0, 0" "1,1,1") false false))))
    (:then_1
      (Default|AddNumber (Variables|Default|GetController) (Variables|Default|GetNumber))
      (Audio|Components|Audio|Play (Variables|Components|Gettypewriter-key-1) 0.0)
      (Audio|Components|Audio|Play (Variables|Components|GetTone) 0.0))))

(event EventTick
  (params (DeltaSeconds :type Float%20%28single-precision%29)))

(fn ConstructionScript
  (Rendering|Components|TextRender|SetText (Variables|Components|GetTextRender) (Variables|Default|GetNumber))
  (Components|StaticMesh|SetStaticMesh (Variables|Components|GetMesh) (Variables|Default|GetButtonMesh))
  (Audio|Components|Audio|SetSound (Variables|Components|GetTone) (Variables|Default|GetSelectedTone)))
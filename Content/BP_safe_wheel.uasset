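; Safe dial actor that a player's hand grabs and twists, active only while IsDoorUnlocked is true.
; Press and Unpress track the grab; Tick adds the hand's world-roll change to the stored rotation to turn the mesh.
; Nearing TargetAngle triggers CorrectPosition, which plays click and latch sounds and unhides the Credits actor.
; A DoOnce and rolling flag gate the looping-style rolling sound during rotation.
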(event Custom|CorrectPosition
  (Utilities|FlowControl|Sequence
    (:then_0
      (Variables|Default|SetIsRollnig false)
      (Utilities|FlowControl|Delay 0.5)
      (Variables|Default|SetIsRollnig true)
      (Utilities|FlowControl|DoOnce false) ; enters at Reset
    )
    (:then_1
      (Audio|Components|Audio|Stop (Variables|Default|GetRollingSound))
      (Audio|Components|Audio|Play (Variables|Default|GetClickSound) 0.0)
      (Utilities|FlowControl|Delay 0.75)
      (Audio|Components|Audio|Play (Variables|Default|GetKa-tching!) 0.0)
      (Rendering|SetActorHiddenInGame (Variables|Default|GetCredits) false))))

(event Custom|Rolling
  (Utilities|FlowControl|DoOnce false))

(event EventBeginPlay)

(event Collision|EventActorBeginOverlap
  (params (OtherActor :type Actor%20Object%20Reference)))

(event EventTick
  (params (DeltaSeconds :type Float%20%28single-precision%29))
  (if (Variables|Default|GetIsDoorUnlocked)
    (if (Variables|Default|GetIsRotating)
      (Utilities|FlowControl|Sequence
        (:then_0
          (bind _output_get (Variables|Default|SetCurrentHandRotation (Math|Rotator|NormalizeAxis (* -1 (.roll (Transformation|GetWorldRotation (Variables|Default|GetPickingHand)))))))
          (bind _output_get_2 (Variables|Default|SetCurrentRelativeRotation (Math|Rotator|NormalizeAxis (+ (- _output_get (Variables|Default|GetInitialHandRotation)) (Variables|Default|GetStartingRelativeRotation)))))
          (Transformation|SetRelativeRotation (Variables|Default|GetStaticMesh) (Math|Rotator|MakeRotator _output_get_2 0.0 0.0) false false)
          (if (Math|Float|NearlyEqual(Float) (Variables|Default|GetCurrentRelativeRotation) (Math|Conversions|ToFloat(Integer) (Variables|Default|GetTargetAngle)) 1.5)
            (CallFunction|CorrectPosition)
            (else
              (Variables|Default|SetIsRollnig true))))
        (:then_1
          (if (Variables|Default|GetIsRollnig)
            (Utilities|FlowControl|DoOnce false :!label _label
              (:Completed
                (Audio|Components|Audio|Play (Variables|Default|GetRollingSound) 0.0)))
            (else
              (Audio|Components|Audio|Stop (Variables|Default|GetRollingSound))))))
      (else
        (Variables|Default|SetIsRollnig false)
        (Audio|Components|Audio|Stop (Variables|Default|GetRollingSound))
        (goto _label Reset)))))

(event EventPress
  (params (ActingHand :type BP%20Motion%20Controller%20Object%20Reference))
  (bind _output_get (Variables|Default|SetPickingHand (Variables|/Game/VirtualRealityBP/Blueprints/BP_MotionController.BP_MotionController_C|GetHandMesh ActingHand)))
  (Variables|Default|SetInitialHandRotation (Math|Rotator|NormalizeAxis (* -1 (.roll (Transformation|GetWorldRotation _output_get)))))
  (Variables|Default|SetIsRotating true))

(event EventUnpress
  (Variables|Default|SetIsRotating false)
  (Variables|Default|SetStartingRelativeRotation (Math|Rotator|NormalizeAxis (.roll (Variables|/Script/Engine.SceneComponent|GetRelativeRotation (Variables|Default|GetStaticMesh))))))

(fn ConstructionScript)